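; BPC_health_component is an actor component that tracks health and applies damage to its owning actor.
; TakeDamage subtracts the incoming amount from Health and broadcasts the OnTakeDamagae dispatcher with that amount.
; When Health reaches zero or below, it broadcasts OnDeath and destroys the owner if DestroyOnDeath is set.
; Health is not clamped, so further hits after death fire OnDeath again.
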(event `TakeDamage`
  (params (DamageTaken :type "Float (double-precision)" :default 1.0))
  (bind _output_get (set `self.health` (- (`self.health`) DamageTaken)))
  (`self.OnTakeDamagae` DamageTaken)
  (if (<= _output_get 0.0)
    (`self.OnDeath`)
    (if (`self.destroy_on_death`)
      (`Actor.K2_DestroyActor` (`self.GetOwner`)))))