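; Level-object component that randomises its owner's static mesh and yaw at BeginPlay for visual variety.
; It targets the first StaticMeshComponent not named "ignore", then optionally swaps in a mesh from the Meshes array and sets a random relative yaw.
; With PositionBasedRandom on, both picks derive from the truncated sum of the actor's location coordinates modulo the range, making results repeatable per position.
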(event `self.ReceiveBeginPlay`
  (`self.SetMeshComponent`))

(event `SetMeshComponent`
  (for _array_element (`Actor.K2_GetComponentsByClass` (`self.GetOwner`) "/Script/Engine.StaticMeshComponent")
    (if (not (== (`KismetSystemLibrary.GetObjectName` _array_element) "ignore"))
      (set `self.mesh` _array_element)
      (`self.Randomise`)
      (break))))

(fn `GetRandomValueBasedOnPosition`
  (params (max :type Integer))
  (returns (output :type Integer))
  (bind (_returnvalue_x _returnvalue_y _returnvalue_z) (`KismetMathLibrary.BreakVector` (`Actor.K2_GetActorLocation` (`self.GetOwner`))))
  (return (`KismetMathLibrary.Abs_Int` (mod (`KismetMathLibrary.FTrunc` (+ _returnvalue_x _returnvalue_y _returnvalue_z)) max))))

(fn `Randomise`
  (`/Engine/EditorBlueprintResources/StandardMacros.IsValid` (`self.mesh`)
    (:`Is Valid`
      (`self.SetMesh`)
      (`self.SetRotation`))))

(fn `SetMesh`
  (bind _meshes (`self.meshes`))
  (if (`self.random_mesh`)
    (`StaticMeshComponent.SetStaticMesh` (`self.mesh`) (select `bool` (`self.position_based_random`) :`false` (`KismetArrayLibrary.Array_Random` _meshes) :`true` (`|GetArrayItem` _meshes (`self.GetRandomValueBasedOnPosition` (`KismetArrayLibrary.Array_Length` _meshes)))))))

(fn `SetRotation`
  (if (`self.random_rotation`)
    (`SceneComponent.K2_SetRelativeRotation` (`self.mesh`) (`KismetMathLibrary.MakeRotator` 0.0 0.0 (`KismetMathLibrary.SelectFloat` (`KismetMathLibrary.Conv_IntToDouble` (`self.GetRandomValueBasedOnPosition` 360)) (`KismetMathLibrary.RandomFloatInRange` 0.0 360.0) (`self.position_based_random`))) false false)))