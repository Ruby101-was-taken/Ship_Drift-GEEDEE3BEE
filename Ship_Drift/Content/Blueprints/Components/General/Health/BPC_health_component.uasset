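; Actor health component that handles damage, death and an optional floating health readout above the owner.
; TakeDamage respects a cooldown between hits, fires damage and death dispatchers, and can destroy the owner on death.
; The health bar is a text render component added at runtime, showing current/max health and turned toward the player camera each tick.
; ResetHealth and Revive restore the starting health, though only ResetHealth refreshes the readout.
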(event `self.ReceiveBeginPlay`
  (bind _output_get (set `self.default_health` (`self.health`)))
  (`KismetSystemLibrary.PrintString` (`KismetStringLibrary.Conv_DoubleToString` _output_get))
  (if (`self.use_health_bar`)
    (`self.AddHealthBar`)))

(event `TakeDamage`
  (params (DamageTaken :type "Float (double-precision)" :default 1.0))
  (if (<= (`self.damage_cooldown`) 0.0)
    (bind _output_get (set `self.health` (- (`self.health`) DamageTaken)))
    (`self.OnTakeDamagae` DamageTaken)
    (`self.UpdateHealthBar`)
    (if (<= _output_get 0.0)
      (`self.OnDeath`)
      (if (`self.destroy_on_death`)
        (`Actor.K2_DestroyActor` (`self.GetOwner`)))
      (else
        (set `self.damage_cooldown` (`self.damage_cooldown_time`))))))

(event `ResetHealth`
  (set `self.health` (`self.default_health`))
  (`self.UpdateHealthBar`))

(event `self.ReceiveTick`
  (params (DeltaSeconds :type "Float (single-precision)"))
  (set `self.damage_cooldown` (- (`self.damage_cooldown`) DeltaSeconds))
  (if (`self.use_health_bar`)
    (`self.LookAtPlayer`)))

(fn `AddHealthBar`
  (bind _text (`self.text`))
  (set `self.spawned_bar` true)
  (bind _returnvalue (`|AddComponentByClass` :`self` (`self.GetOwner`) :`Class` "/Script/Engine.TextRenderComponent"))
  (bind _output_get (set `self.text` _returnvalue))
  (`self.K2_SetRelativeLocation` _output_get (+ (`SceneComponent.RelativeLocation` _output_get) (`self.bar_offset`)) false false)
  (`TextRenderComponent.SetHorizontalAlignment` _text "EHTA_Center")
  (`TextRenderComponent.SetWorldSize` _text (`self.text_size`))
  (`self.UpdateHealthBar`))

(fn `IsAlive`
  (returns (alive :type Boolean))
  (return (> (`self.health`) 0.0)))

(fn `LookAtPlayer`
  (bind _text (`self.text`))
  ; rotates the text to face the world camera
  (`self.K2_SetWorldRotation` _text (`KismetMathLibrary.FindLookAtRotation` (`self.K2_GetComponentLocation` _text) (`self.K2_GetComponentLocation` (`PlayerCameraManager.TransformComponent` (`GameplayStatics.GetPlayerCameraManager` 0)))) false false))

(fn `Revive`
  (set `self.health` (`self.default_health`)))

(fn `UpdateHealthBar`
  (if (`self.spawned_bar`)
    (`TextRenderComponent.K2_SetText` (`self.text`) (`KismetTextLibrary.Conv_StringToText` (`KismetStringLibrary.Concat_StrStr` (`KismetStringLibrary.Conv_Int64ToString` (`KismetMathLibrary.FTrunc64` (`self.health`))) "/" (`KismetStringLibrary.Conv_Int64ToString` (`KismetMathLibrary.FTrunc64` (`self.default_health`))))))))