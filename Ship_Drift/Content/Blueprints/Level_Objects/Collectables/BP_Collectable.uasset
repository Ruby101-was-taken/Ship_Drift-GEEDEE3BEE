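; Collectable scrap pickup that adds to the player's scrap count when the player collides with it.
; On BeginPlay it caches the level's BP_Score_Manager and attempts to spawn via AttemptSpawn, which Reset calls again while re-enabling pickup.
; A valid pickup increments scrap on the manager, then makes the object inaccessible, guarded by CanBePickedUp.
; Accessibility overrides extend the parent's behavior by toggling mesh visibility, so the actor is hidden rather than destroyed.
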(event `self.ReceiveBeginPlay`
  (bind _outactors (`GameplayStatics.GetAllActorsOfClass` "/Game/Blueprints/Managers/Score/BP_Score_Manager.BP_Score_Manager_C"))
  (set `self.score_manager` (`|GetArrayItem` _outactors))
  (set `self.spawned_z` 0.0)
  (`self.AttemptSpawn`))

(event `/Game/Blueprints/Interfaces/BPI_Resetable.Reset`
  (params (level_type :type "/Game/Blueprints/Enum/Levels/Types/E_Level_Types Enum" :default "NewEnumerator0") (weather_type :type "/Game/Blueprints/Enum/Levels/Types/E_Weather_Types Enum" :default "NewEnumerator0"))
  (`self.AttemptSpawn`)
  (set `self.can_be_picked_up` true))

(fn `MakeObjectAccessable`
  (`parent.MakeObjectAccessable`)
  (`SceneComponent.SetVisibility` (`self.StaticMesh`) true false))

(fn `MakeObjectInaccessable`
  (`parent.MakeObjectInaccessable`)
  (`SceneComponent.SetVisibility` (`self.StaticMesh`) false false))

(fn `OnCollideWithPlayer`
  (if (`self.can_be_picked_up`)
    (`/Game/Blueprints/Managers/Score/BP_Score_Manager.IncermentScrap` (`self.score_manager`))
    (`self.MakeObjectInaccessable`)
    (set `self.can_be_picked_up` false)))

(fn `UserConstructionScript`)