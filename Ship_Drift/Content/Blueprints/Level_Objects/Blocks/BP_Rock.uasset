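; BP_Rock is a rock block level object that varies its appearance per instance.
; Its construction script picks a random mesh from the Mesh array, calls MakeObjectAccessable, and yaws the static mesh randomly within RotationRange.
; On BeginPlay it reapplies its transform with only X and Y location carried over, leaving Z at the pin default.
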(event `self.ReceiveBeginPlay`
  (bind _returnvalue (`self.GetTransform`))
  (`self.K2_SetActorTransform` (`KismetMathLibrary.MakeTransform` (`KismetMathLibrary.MakeVector` (.x (.location _returnvalue)) (.y (.location _returnvalue))) (.rotation _returnvalue) (.scale _returnvalue))))

(fn `UserConstructionScript`
  (bind (_x _y) (`KismetMathLibrary.BreakVector2D` (`self.RotationRange`)))
  (`StaticMeshComponent.SetStaticMesh` (`self.StaticMesh`) (`KismetArrayLibrary.Array_Random` (`self.Mesh`)))
  (`self.MakeObjectAccessable`)
  (`SceneComponent.K2_SetRelativeRotation` (`self.StaticMesh`) (`KismetMathLibrary.MakeRotator` 0.0 0.0 (`KismetMathLibrary.RandomFloatInRange` _x _y)) false false))