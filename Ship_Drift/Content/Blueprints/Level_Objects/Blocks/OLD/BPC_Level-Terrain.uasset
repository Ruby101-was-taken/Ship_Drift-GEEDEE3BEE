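; Level terrain block component that sets a static mesh for a forced or random category and spawns actors around it.
; SpawnBlock resolves the type, recursively rerolling two excluded values, then looks up that type's row in the Meshes data table, falling back to a cone.
; Mesh, spawnable classes and offsets come from separately re-evaluated random picks, so they can mismatch.
; Spawned actors use shuffled offsets and are tracked for removal.
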(event `SpawnBlock`
  (params (PossibleCategories :type "Array of /Game/Blueprints/Enum/Levels/Blocks/E_Block_Categories Enum") (ForceType :type "/Game/Blueprints/Enum/Levels/Blocks/E_Block_Categories Enum" :default "NewEnumerator0") (Position :type "Transform Structure"))
  (set `self.possible_categories` PossibleCategories)
  (bind _output_get (set `self.type` ForceType))
  (if (`|EnumEquality` _output_get "NewEnumerator5")
    (`self.SetType`))
  (bind _mesh (`self.GetMesh` Position))
  (`self.SetMesh` _mesh))

(fn `GetMesh`
  (params (Position :type "Transform Structure"))
  (returns (Mesh :type "StaticMesh Object Reference"))
  (bind _returnvalue (`KismetStringLibrary.Conv_StringToName` (`|GetEnumeratorNameAsString` (`self.type`))))
  (bind _returnvalue_2 (`|GetDataTableRow` (`self.meshes`) _returnvalue)
    (:`then`
      (bind _outitem (`KismetArrayLibrary.Array_Random` (`.Models_6_3CC7D668444355880C502FB980D81955` (break `/Game/Blueprints/Structs/Level/Blocks/S_Level_Block_Models` (`BlueprintMapLibrary.Map_Find` (`.Models_8_07DF146A4EEDA745E22355BFFC0286C0` (break `/Game/Blueprints/Structs/Level/Blocks/S_Level_Block_Type` _returnvalue_2)) (cast `/Game/Blueprints/Enum/Levels/Blocks/E_Block_Types` (`KismetMathLibrary.Conv_IntToByte` (`KismetMathLibrary.RandomIntegerInRange` 0 (- (enumcount `/Game/Blueprints/Enum/Levels/Blocks/E_Block_Types`) 1)))))))))
      (`self.SpawnBPs` (`.Spawnables_12_E932E011497664A8C53AC1AA257AD328` (break `/Game/Blueprints/Structs/Level/Blocks/S_Level_Block_Model_Info` _outitem)) (`.Positions_16_90E05E0F415099DE53D22FA335C98B2D` (break `/Game/Blueprints/Structs/Level/Blocks/S_Level_Block_Model_Info` _outitem)) (+ Position_Location (0.0 0.0 -900.0)))
      (return (break `/Game/Blueprints/Structs/Level/Blocks/S_Level_Block_Model_Info` _outitem)))
    (:`RowNotFound`
      (`KismetSystemLibrary.PrintString` (`KismetStringLibrary.Conv_NameToString` _returnvalue))
      (return "/Engine/BasicShapes/Cone.Cone"))))

(fn `RemoveSpawnedActors`
  (for _array_element (`self.spawned_actors`)
    (`/Engine/EditorBlueprintResources/StandardMacros.IsValid` _array_element
      (:`Is Valid`
        (`Actor.K2_DestroyActor` _array_element))))
  (`KismetArrayLibrary.Array_Clear` (`self.spawned_actors`)))

(fn `SetMesh`
  (params (Mesh :type "StaticMesh Object Reference"))
  (`self.SetStaticMesh` Mesh))

(fn `SetType`
  (bind _output_get (set `self.type` (`KismetArrayLibrary.Array_Random` (`self.possible_categories`))))
  (if (or (`|EnumEquality` _output_get "NewEnumerator4") (`|EnumEquality` _output_get "NewEnumerator5"))
    (`self.SetType`)))

(fn `SpawnBPs`
  (params (Classes :type "Array of Actor Class Reference") (Offset :type "Array of Vector Structure") (Position :type "Vector Structure"))
  (`KismetArrayLibrary.Array_Shuffle` Offset)
  (for _index (range (+ (`KismetMathLibrary.RandomInteger` (`KismetArrayLibrary.Array_Length` Offset)) 1))
    (bind _returnvalue (`|SpawnActorFromClass` (`KismetArrayLibrary.Array_Random` Classes) (`KismetMathLibrary.MakeTransform` (+ (`|GetArrayItem` Offset _index) Position)) "Undefined" "MultiplyWithRoot" null null))
    (`KismetArrayLibrary.Array_Add` (`self.spawned_actors`) _returnvalue)))