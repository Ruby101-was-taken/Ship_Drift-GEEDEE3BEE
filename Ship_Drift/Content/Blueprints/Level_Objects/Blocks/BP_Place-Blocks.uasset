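; Level block placer that builds a grid of BP_LevelBlock actors and rebuilds it with a new level type on reset.
; Place forces a special type at the origin and another on the back and side edges, then spawns each block using the allowed categories.
; ResetLevel advances a random look-ahead queue of level types, reads that type's categories from a data table, destroys old blocks and places again.
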(event `self.ReceiveBeginPlay`)

(event `Place`
  (bind _interval (`self.interval`))
  (bind _returnvalue (/ (`self.width`) 2))
  (set `self.should_be_full` false)
  (for _index (range -1 (`self.depth`))
    (set `self.x` _index)
    (for _index_2 (range (- 0 _returnvalue) (+ _returnvalue 1))
      (set `self.z` _index_2)
      (bind _returnvalue_2 (`KismetMathLibrary.Conv_IntToDouble` (* _index _interval)))
      (bind _returnvalue_3 (`KismetMathLibrary.Conv_IntToDouble` (* _index_2 _interval)))
      (bind _returnvalue_4 (`|SpawnActorFromClass` "/Game/Blueprints/Level_Objects/Blocks/BP_Level-Block.BP_Level-Block_C" (`KismetMathLibrary.MakeTransform` (`KismetMathLibrary.MakeVector` _returnvalue_2 _returnvalue_3 (`KismetMathLibrary.Conv_IntToDouble` (/ _interval 2)))) "Undefined" "MultiplyWithRoot" null null))
      (if (and (== _returnvalue_2 0.0) (== _returnvalue_3 0.0))
        (set `/Game/Blueprints/Level_Objects/Blocks/BP_Level-Block.force_type` "NewEnumerator6" _returnvalue_4)
        (else
          (bind _full (`self.ShouldBeFull` (`self.x`) (`self.z`) (`self.width`)))
          (if _full
            (set `/Game/Blueprints/Level_Objects/Blocks/BP_Level-Block.force_type` "NewEnumerator4" _returnvalue_4))))
      (`/Game/Blueprints/Level_Objects/Blocks/BP_Level-Block.Spawn` _returnvalue_4 (`self.allowed_types`))
      (`KismetArrayLibrary.Array_Add` (`self.level_Blocks`) _returnvalue_4))))

(event `ResetLevel`
  (bind _level_blocks (`self.level_Blocks`))
  (`self.IncrementLevelType`)
  ; Remove all old blocks
  (for _array_element _level_blocks
    (`self.K2_DestroyActor` _array_element))
  (`KismetArrayLibrary.Array_Clear` _level_blocks)
  (`self.Place`))

(fn `GetRandomLevelType`
  (returns (Type :type "/Game/Blueprints/Enum/Levels/Types/E_Level_Types Enum"))
  (return (cast `/Game/Blueprints/Enum/Levels/Types/E_Level_Types` (`KismetMathLibrary.Conv_IntToByte` (`KismetMathLibrary.RandomIntegerInRange` 0 (- (enumcount `/Game/Blueprints/Enum/Levels/Types/E_Level_Types`) 1))))))

(fn `IncrementLevelType`
  (for _ (range (`KismetArrayLibrary.Array_Length` (`self.future_level_types`)) (+ (`self.level_look_ahead_length`) 1))
    (`KismetArrayLibrary.Array_Add` (`self.future_level_types`) (`self.GetRandomLevelType`)))
  (bind _output_get (set `self.current_level_type` (`|GetArrayItem` (`self.future_level_types`))))
  (`KismetSystemLibrary.PrintString` "Current:" true true (struct :`G` 0.66 :`B` 1.0 :`A` 1.0) 10.0)
  (`KismetSystemLibrary.PrintString` (`|GetEnumeratorNameAsString` _output_get) true true (struct :`G` 0.66 :`B` 1.0 :`A` 1.0) 10.0)
  (`self.SetAllowedTypes`)
  (`KismetArrayLibrary.Array_Remove` (`self.future_level_types`))
  (`KismetSystemLibrary.PrintString` "Future Types:" true true (struct :`G` 0.66 :`B` 1.0 :`A` 1.0) 10.0)
  (for _array_element (`self.future_level_types`)
    (`KismetSystemLibrary.PrintString` (`|GetEnumeratorNameAsString` _array_element) true true (struct :`G` 0.66 :`B` 1.0 :`A` 1.0) 10.0)))

(fn `SetAllowedTypes`
  (bind _returnvalue (`|GetDataTableRow` (`self.level_block_categories`) (`KismetStringLibrary.Conv_StringToName` (`|GetEnumeratorNameAsString` (`self.current_level_type`))))
    (:`then`
      (set `self.allowed_types` (`.Allowed_Categories_3_9971F99D4F7CCFF9780E3B9DA4CC5EE9` (break `/Game/Blueprints/Structs/Level/Types/S_Level_Allowed_Block_Categories` _returnvalue))))))

(fn `ShouldBeFull`
  (params (x :type Integer) (z :type Integer) (width :type Integer))
  (returns (Full :type Boolean))
  (bind _returnvalue (or (== x -1) (== (`KismetMathLibrary.Abs_Int` z) (/ width 2))))
  (if _returnvalue
    _
    (else
      _))
  (return _returnvalue))

(fn `UserConstructionScript`)