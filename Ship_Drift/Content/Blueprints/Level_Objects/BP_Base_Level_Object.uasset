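; BP_Base_Level_Object is a base for level objects that randomly appear per level type and react when the player overlaps them.
; AttemptSpawn looks up spawn conditions for the level type, falling back to the default type, then rolls a forced or percentage chance.
; Rather than spawning or destroying, it moves the actor to an accessible height or far below the level out of reach.
; Player overlaps call OnCollideWithPlayer, left empty here.
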(event `self.ReceiveActorBeginOverlap`
  (params (OtherActor :type "Actor Object Reference"))
  (if (== (`GameplayStatics.GetObjectClass` OtherActor) "/Game/Blueprints/Player/BP_Player.BP_Player_C")
    (bind _asbp_player (cast `/Game/Blueprints/Player/BP_Player` OtherActor))
    (`self.OnCollideWithPlayer` _asbp_player)))

(fn `AttemptSpawn`
  (params (level_type :type "/Game/Blueprints/Enum/Levels/Types/E_Level_Types Enum" :default "NewEnumerator0"))
  (`self.FindAndSetConditions` level_type)
  ; if sould always spawn
  (if (`self.forced_spawn`)
    (`self.MakeObjectAccessable` :!label _label)
    (else
      ; if object randomly can spawn
      (if (>= (`self.spawn_chance`) (`KismetMathLibrary.RandomFloatInRange` 1.0 100.0))
        (goto _label)
        (else
          (`self.MakeObjectInaccessable`))))))

(fn `FindAndSetConditions`
  (params (level_type :type "/Game/Blueprints/Enum/Levels/Types/E_Level_Types Enum" :default "NewEnumerator0"))
  (bind (_value _returnvalue) (`BlueprintMapLibrary.Map_Find` (`self.spawn_conditions`) level_type))
  (bind (_forced_spawn _spawn_chance) (break `/Game/Blueprints/Structs/Level/Blocks/S_Spawn_Conditions` _value))
  ; Attempt to get the current level type's conditions
  (if _returnvalue
    (`self.SetConditions` _forced_spawn _spawn_chance)
    (else
      ; As a fall back, get the default type conditions, unless we are already looking for that type
      (if (`|EnumEquality` level_type "NewEnumerator0")
        ; If not conditions are found, just don't allow object to spawn
        (`self.SetConditions` false)
        (else
          (`self.FindAndSetConditions` "NewEnumerator0"))))))

(fn `MakeObjectAccessable`
  (bind _returnvalue (`self.GetTransform`))
  (`self.K2_SetActorLocation` (`KismetMathLibrary.MakeVector` (.x (.location _returnvalue)) (.y (.location _returnvalue)) (`self.accessable_height`))))

(fn `MakeObjectInaccessable`
  (bind _returnvalue (`self.GetTransform`))
  ; moves object so far down it can't be reached
  (`self.K2_SetActorLocation` (`KismetMathLibrary.MakeVector` (.x (.location _returnvalue)) (.y (.location _returnvalue)) -10000.0)))

(fn `OnCollideWithPlayer`
  (params (player :type "/Game/Blueprints/Player/BP_Player Object Reference")))

(fn `SetConditions`
  (params (force_spawn :type Boolean) (spawn_chance :type "Float (double-precision)"))
  (set `self.forced_spawn` force_spawn)
  (set `self.spawn_chance` spawn_chance))

(fn `UserConstructionScript`)