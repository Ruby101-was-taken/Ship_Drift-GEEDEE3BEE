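; Trigger volume that detects when the player inside it has been facing against a set direction for too long.
; While colliding, Tick compares the player's forward vector to Direction with a dot product.
; Facing away raises a wrong-way timer stored on the player, and any other heading lowers it.
; Once the timer reaches the player's threshold, it calls OnFaceWrongWay every tick, an empty function here.
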(event `self.ReceiveTick`
  (params (DeltaSeconds :type "Float (single-precision)"))
  (bind (_returnvalue_location _returnvalue_rotation) (`KismetMathLibrary.BreakTransform` (`self.GetTransform` (`self.player`))))
  (if (`self.colliding`)
    (if (< (`KismetMathLibrary.Dot_VectorVector` (`KismetMathLibrary.Normal` (`KismetMathLibrary.GetForwardVector` _returnvalue_rotation)) (`self.direction`)) -0.5)
      (`self.FacingWrongWay` DeltaSeconds)
      (else
        (`self.FacingRightWay` DeltaSeconds)))))

(fn `FacingRightWay`
  (params (delta_seconds :type "Float (double-precision)"))
  (if (not (<= (`/Game/Blueprints/Player/BP_Player.wrong_way_timer` (`self.player`)) 0.0))
    (set `/Game/Blueprints/Player/BP_Player.wrong_way_timer` (- (`/Game/Blueprints/Player/BP_Player.wrong_way_timer` (`self.player`)) delta_seconds) (`self.player`))))

(fn `FacingWrongWay`
  (params (delta_seconds :type "Float (double-precision)"))
  (bind _player (`self.player`))
  (if (>= (`/Game/Blueprints/Player/BP_Player.wrong_way_timer` _player) (`/Game/Blueprints/Player/BP_Player.wrong_way_threshold` _player))
    (`self.OnFaceWrongWay`)
    (else
      (set `/Game/Blueprints/Player/BP_Player.wrong_way_timer` (+ (`/Game/Blueprints/Player/BP_Player.wrong_way_timer` (`self.player`)) delta_seconds) (`self.player`)))))

(fn `OnCollideWithPlayer`
  (params (player :type "/Game/Blueprints/Player/BP_Player Object Reference"))
  (set `self.player` player)
  (set `self.colliding` true))

(fn `OnFaceWrongWay`)

(fn `OnLeaveCollideWithPlayer`
  (params (player :type "/Game/Blueprints/Player/BP_Player Object Reference"))
  (set `self.colliding` false))

(fn `UserConstructionScript`)