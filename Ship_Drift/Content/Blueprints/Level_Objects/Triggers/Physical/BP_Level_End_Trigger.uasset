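; Level end trigger, a resettable level object with a health bar that stops the score timer when it becomes inaccessible.
; Reset attempts a spawn for the given level and test type, while SimpleReset makes it accessible again; both then refresh the health bar.
; The MakeObjectInaccessable override runs the parent logic, then pauses the timer on BP_Score_Manager.
; A call to reset the level through BP_Level_Reset_Manager is left unconnected.
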(event `/Game/Blueprints/Interfaces/BPI_Resetable.Reset`
  (params (level_type :type "/Game/Blueprints/Enum/Levels/Types/E_Level_Types Enum" :default "NewEnumerator0") (wind :type "Vector Structure") (weather :type "/Game/Blueprints/Enum/Levels/Types/E_Weather_Types Enum" :default "NewEnumerator0") (test_type :type "/Game/Blueprints/Enum/Testing/E_Tester_Type Enum" :default "NewEnumerator0"))
  (`self.AttemptSpawn` level_type test_type)
  (`/Game/Blueprints/Components/General/Health/BPC_health_component.UpdateHealthBar` (`self.BPC_health_component`) :!label _label))

(event `/Game/Blueprints/Interfaces/BPI_Resetable.SimpleReset`
  (`self.MakeObjectAccessable`)
  (goto _label))

(fn `MakeObjectInaccessable`
  (`parent.MakeObjectInaccessable`)
  (bind _outactors (`GameplayStatics.GetAllActorsOfClass` "/Game/Blueprints/Managers/Score/BP_Score_Manager.BP_Score_Manager_C"))
  (set `/Game/Blueprints/Managers/Score/BP_Score_Manager.pause_timer` true (`|GetArrayItem` _outactors)))

(fn `UserConstructionScript`)