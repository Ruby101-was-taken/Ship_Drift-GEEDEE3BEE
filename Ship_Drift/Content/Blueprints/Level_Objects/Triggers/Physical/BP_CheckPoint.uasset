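; BP_CheckPoint is a checkpoint trigger with a rope strung across a configurable width.
; The construction script positions the Left and Right components, the rope end and the collision box from Width.
; On player collision it passes its location to the player's HitCheckpoint and hides the rope.
; Reset calls AttemptSpawn with the level type, and the MakeObjectAccessable override shows the rope again.
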(event `/Game/Blueprints/Interfaces/BPI_Resetable.Reset`
  (params (level_type :type "/Game/Blueprints/Enum/Levels/Types/E_Level_Types Enum" :default "NewEnumerator0") (wind :type "Vector Structure") (weather :type "/Game/Blueprints/Enum/Levels/Types/E_Weather_Types Enum" :default "NewEnumerator0"))
  (`self.AttemptSpawn` level_type))

(fn `MakeObjectAccessable`
  (`parent.MakeObjectAccessable`)
  (`SceneComponent.SetVisibility` (`self.Rope`) true false))

(fn `OnCollideWithPlayer`
  (params (player :type "/Game/Blueprints/Player/BP_Player Object Reference"))
  (`/Game/Blueprints/Player/BP_Player.HitCheckpoint` player (`self.K2_GetActorLocation`))
  (`SceneComponent.SetVisibility` (`self.Rope`) false false))

(fn `UserConstructionScript`
  (bind _rope (`self.Rope`))
  (bind _returnvalue (/ (`self.width`) 2.0))
  (bind _returnvalue_2 (/ (`self.width`) 2.0))
  (bind _relativelocation_x (`KismetMathLibrary.BreakVector` (`SceneComponent.RelativeLocation` _rope)))
  (`parent.UserConstructionScript`)
  (`SceneComponent.K2_SetRelativeLocation` (`self.Right`) (`KismetMathLibrary.MakeVector` 0.0 (* _returnvalue -1.0)) false false)
  (`SceneComponent.K2_SetRelativeLocation` (`self.Left`) (`KismetMathLibrary.MakeVector` 0.0 _returnvalue) false false)
  (set `CableComponent.EndLocation` (`KismetMathLibrary.MakeVector` _relativelocation_x _returnvalue_2) _rope)
  (`BoxComponent.SetBoxExtent` (`self.Box`) (`KismetMathLibrary.MakeVector` 100.0 _returnvalue_2 100.0) true))