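; BP_Mine is a floating sea mine level object that kills the player's skipper on contact.
; It bobs via a water float component and uses inherited spawn logic on begin play and level reset.
; Collision spawns a Niagara explosion and sound, applies overwhelming damage, and swaps mesh visibility for an Explosion component.
; Simple reset and MakeObjectAccessable restore the intact mine by reversing that visibility swap.
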(event `self.ReceiveBeginPlay`
  (bind _bpc_water_float_component (`self.BPC_Water_Float_Component`))
  (`/Game/Blueprints/Components/Animation/BPC_Water_Float_Component.SetMesh` _bpc_water_float_component (`self.Mesh`))
  (`/Game/Blueprints/Components/Animation/BPC_Water_Float_Component.EnableBob` _bpc_water_float_component)
  (`self.AttemptSpawn` "NewEnumerator0"))

(event `/Game/Blueprints/Interfaces/BPI_Resetable.Reset`
  (params (level_type :type "/Game/Blueprints/Enum/Levels/Types/E_Level_Types Enum" :default "NewEnumerator0") (wind :type "Vector Structure") (weather :type "/Game/Blueprints/Enum/Levels/Types/E_Weather_Types Enum" :default "NewEnumerator0"))
  (`self.AttemptSpawn` level_type))

(event `/Game/Blueprints/Interfaces/BPI_Resetable.SimpleReset`
  (`self.SetExplosion` false))

(fn `MakeObjectAccessable`
  (`parent.MakeObjectAccessable`)
  (`self.SetExplosion` false))

(fn `OnCollideWithPlayer`
  (params (player :type "/Game/Blueprints/Player/BP_Player Object Reference"))
  (`NiagaraFunctionLibrary.SpawnSystemAtLocation` "/Game/FX/NS_Explosion.NS_Explosion" (`self.K2_GetActorLocation`))
  ; Just hit it with a ton of damage. We are killing skipper with this one lads
  (`GameplayStatics.ApplyDamage` player 10000.0)
  (`self.SetExplosion` true)
  (`GameplayStatics.PlaySoundAtLocation` "/Game/Sound/SoundCue/Objects/A_Mine_Cue.A_Mine_Cue" (`self.K2_GetActorLocation`) (struct) 1.0 1.0 0.0 null null null null))

(fn `SetExplosion`
  (params (on_or_off :type Boolean))
  (`SceneComponent.SetVisibility` (`self.Explosion`) on_or_off false)
  (`SceneComponent.SetVisibility` (`self.Mesh`) (not on_or_off) false))

(fn `UserConstructionScript`
  (`parent.UserConstructionScript`))