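; BP_Rammable is a destructible level object that the player breaks by ramming it or hitting it with cannonballs.
; Both attacks damage its health component; death plays a breaking sound and explosion, then makes it inaccessible until MakeObjectAccessable revives it.
; A ram cancels the player's harpoon, and if the object survives, it bounces the player back with a minimum-strength impulse, calls the empty OnRam hook and consumes the ram.
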(event `self.Trigger.OnComponentBeginOverlap`
  (params (OverlappedComponent :type "PrimitiveComponent Object Reference") (OtherActor :type "Actor Object Reference") (OtherComp :type "PrimitiveComponent Object Reference") (OtherBodyIndex :type Integer) (bFromSweep :type Boolean) (SweepResult :type "HitResult Structure (by ref)"))
  ; Deal damage from cannon fire
  (bind _asbp_player_cannon_ball (cast `/Game/Blueprints/Player/Weapons/BP_Player_CannonBall` OtherActor))
  (`/Game/Blueprints/Components/General/Health/BPC_health_component.TakeDamage` (`self.BPC_health_component`) (`/Game/Blueprints/Player/Weapons/BP_Player_CannonBall.damage` _asbp_player_cannon_ball)))

(event `self.BPC_health_component.OnDeath`
  (bind _returnvalue (`self.K2_GetActorLocation`))
  (`GameplayStatics.PlaySoundAtLocation` "/Game/Sound/SoundCue/Objects/A_Barrier_Breaking_Cue.A_Barrier_Breaking_Cue" _returnvalue (struct) 1.0 1.0 0.0 null null null null)
  (`NiagaraFunctionLibrary.SpawnSystemAtLocation` "/Game/FX/NS_Explosion.NS_Explosion" _returnvalue (struct) (2.0 4.0 2.0))
  (`self.MakeObjectInaccessable`))

(fn `CheckImpluseStrength`
  (params (in_impulse :type "Vector Structure"))
  (returns (out_impulse :type "Vector Structure"))
  (if (< (`KismetMathLibrary.VSize` in_impulse) (`self.minimum_impluse`))
    (return (* (`KismetMathLibrary.Normal` in_impulse) (`self.minimum_impluse`)))
    (else
      (return in_impulse))))

(fn `MakeObjectAccessable`
  (`parent.MakeObjectAccessable`)
  (`/Game/Blueprints/Components/General/Health/BPC_health_component.Revive` (`self.BPC_health_component`)))

(fn `OnCollideWithPlayer`
  (params (player :type "/Game/Blueprints/Player/BP_Player Object Reference"))
  (bind (_damage _velocity) (`/Game/Blueprints/Player/BP_Player.GetRamHitPower` player))
  (`/Game/Blueprints/Components/General/Health/BPC_health_component.TakeDamage` (`self.BPC_health_component`) _damage)
  (`/Game/Blueprints/Player/BP_Player.CancelHarpoon` player)
  (if (`/Game/Blueprints/Components/General/Health/BPC_health_component.IsAlive` (`self.BPC_health_component`))
    (`CharacterMovementComponent.AddImpulse` (`Character.CharacterMovement` player) (`self.CheckImpluseStrength` (* _velocity (* (`self.ram_recoil`) -1.0))) true)
    (`self.OnRam` player _damage)
    (`/Game/Blueprints/Player/BP_Player.UseRam` player _damage)))

(fn `OnRam`
  (params (player :type "/Game/Blueprints/Player/BP_Player Object Reference") (power :type "Float (double-precision)")))

(fn `UserConstructionScript`)