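; BP_Barrier is a breakable level object that attempts to spawn on BeginPlay and again on Reset, which also refreshes its health bar.
; When its health component reports death, it makes itself inaccessible and plays a breaking sound.
; It extends the parent's MakeObjectAccessable by scaling the Solid component's X axis to Width.
; Being rammed only plays a second breaking sound, ignoring the player and power inputs.
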(event `self.ReceiveBeginPlay`
  (`self.AttemptSpawn` "NewEnumerator0"))

(event `self.BPC_health_component.OnDeath`
  (`self.MakeObjectInaccessable`)
  (`GameplayStatics.PlaySound2D` "/Game/Sound/WavFiles/Level_Objects/Barrier/MSW_Barrier_Breaking_Ver1.MSW_Barrier_Breaking_Ver1" 1.0 1.0 0.0 null null))

(event `/Game/Blueprints/Interfaces/BPI_Resetable.Reset`
  (params (level_type :type "/Game/Blueprints/Enum/Levels/Types/E_Level_Types Enum" :default "NewEnumerator0") (wind :type "Vector Structure") (weather :type "/Game/Blueprints/Enum/Levels/Types/E_Weather_Types Enum" :default "NewEnumerator0"))
  (`self.AttemptSpawn` "NewEnumerator0")
  (`/Game/Blueprints/Components/General/Health/BPC_health_component.UpdateHealthBar` (`self.BPC_health_component`)))

(fn `MakeObjectAccessable`
  (bind _returnvalue (`SceneComponent.GetRelativeTransform` (`self.Solid`)))
  (`parent.MakeObjectAccessable`)
  (`SceneComponent.SetRelativeScale3D` (`self.Solid`) (`KismetMathLibrary.MakeVector` (`self.width`) (.y (.scale _returnvalue)) (.z (.scale _returnvalue)))))

(fn `OnRam`
  (params (player :type "/Game/Blueprints/Player/BP_Player Object Reference") (power :type "Float (double-precision)"))
  (`GameplayStatics.PlaySound2D` "/Game/Sound/WavFiles/Level_Objects/Barrier/MSW_Barrier_Breaking_Ver2.MSW_Barrier_Breaking_Ver2" 1.0 1.0 0.0 null null))

(fn `UserConstructionScript`
  (`parent.UserConstructionScript`))