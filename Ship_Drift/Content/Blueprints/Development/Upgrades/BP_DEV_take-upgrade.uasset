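; BP_DEV_take-upgrade is a development actor that removes a configured upgrade from the player.
; On BeginPlay it caches the first BP_Player found, writes UpgradeType onto its west and east text labels, and draws a long-lasting debug box at its root.
; Any actor overlap calls RemoveUpgrade with that type on the cached player, without checking which actor triggered it.
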(event `self.ReceiveBeginPlay`
  (bind _returnvalue (`KismetTextLibrary.Conv_StringToText` (`self.upgrade_type`)))
  (bind _outactors (`GameplayStatics.GetAllActorsOfClass` "/Game/Blueprints/Player/BP_Player.BP_Player_C"))
  (set `self.player` (`|GetArrayItem` _outactors))
  (`TextRenderComponent.K2_SetText` (`self.Upgrade Name West`) _returnvalue)
  (`TextRenderComponent.K2_SetText` (`self.Upgrade Name East`) _returnvalue)
  (`KismetSystemLibrary.DrawDebugBox` (`SceneComponent.K2_GetComponentLocation` (`self.DefaultSceneRoot`)) (100.0 100.0 100.0) (struct) (struct) 1000.0))

(event `self.ReceiveActorBeginOverlap`
  (params (OtherActor :type "Actor Object Reference"))
  (bind _player (`self.player`))
  (if (`KismetSystemLibrary.IsValid` _player)
    (`/Game/Blueprints/Player/BP_Player.Remove Upgrade` _player (`self.upgrade_type`))))

(fn `UserConstructionScript`)