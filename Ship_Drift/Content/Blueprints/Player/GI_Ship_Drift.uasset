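; Game instance for Ship Drift that owns the BP_SaveGame data and handles loading and saving it to a single slot.
; Init synchronously loads or creates the save object, sets NewGame to true on every launch and writes it back.
; Load and save events offer sync or async paths, though only async loading of an existing save calls OnGameLoaded.
; SavePlayer stores player data before saving, and GetGameData exposes the cached object.
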(event `self.ReceiveInit`
  ; Initialize
  (`/Game/Blueprints/Interfaces/BPI_SaveGame.LoadGameData` false)
  (set `/Game/Data/Game/BP_SaveGame.new_game` true (`self.saved_data`))
  (`/Game/Blueprints/Interfaces/BPI_SaveGame.SaveGameData` false))

(event `/Game/Blueprints/Interfaces/BPI_SaveGame.LoadGameData`
  (params (async :type Boolean))
  ;[0.02673 0.15 0 0.5] Load Game
  (bind _returnvalue (`GameplayStatics.DoesSaveGameExist` (`self.slot_name`)))
  (if _returnvalue
    (if async
      (bind _savegame (`AsyncActionHandleSaveGame.AsyncLoadGameFromSlot` (`self.slot_name`))
        (:`Completed`
          (bind _asbp_save_game (cast `/Game/Data/Game/BP_SaveGame` _savegame))
          (set `self.saved_data` _asbp_save_game)
          (`self.On Game Loaded`)))
      (else
        (bind _returnvalue_2 (`GameplayStatics.LoadGameFromSlot` (`self.slot_name`)))
        (bind _asbp_save_game_2 (cast `/Game/Data/Game/BP_SaveGame` _returnvalue_2))
        (set `self.saved_data` _asbp_save_game_2)))
    (else
      (bind _returnvalue_3 (`GameplayStatics.CreateSaveGameObject` "/Game/Data/Game/BP_SaveGame.BP_SaveGame_C"))
      (set `self.saved_data` _returnvalue_3))))

(event `/Game/Blueprints/Interfaces/BPI_SaveGame.SaveGameData`
  (params (async :type Boolean))
  ;[0.09476 7.3e-05 0.15 0.5] Save Game
  (if async
    (`AsyncActionHandleSaveGame.AsyncSaveGameToSlot` (`self.saved_data`) (`self.slot_name`))
    (else
      (`GameplayStatics.SaveGameToSlot` (`self.saved_data`) (`self.slot_name`)))))

(event `/Game/Blueprints/Interfaces/BPI_SaveGame.SavePlayer`
  (params (player_save :type "/Game/Blueprints/Structs/Player/S_Player_Save Structure") (async :type Boolean))
  ; Save Player
  (set `/Game/Data/Game/BP_SaveGame.player_save` player_save (`self.saved_data`))
  (`/Game/Blueprints/Interfaces/BPI_SaveGame.SaveGameData` async))

(fn `GetGameData`
  (returns (save_game_data :type "/Game/Data/Game/BP_SaveGame Object Reference"))
  (return (`self.saved_data`)))