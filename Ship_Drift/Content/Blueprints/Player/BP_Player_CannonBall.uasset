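; Player cannonball projectile that flies along a set direction for a limited lifetime.
; On BeginPlay it reads Speed and Duration from the data table row referenced by CannonInfo.
; Each Tick it offsets itself by Direction times Speed without sweeping, so movement is per frame rather than scaled by delta time.
; It counts the lifetime down by delta seconds and destroys itself when it runs out.
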(event `self.ReceiveBeginPlay`
  (bind (_cannon_info_datatable _cannon_info_rowname) (break `DataTableRowHandle` (`self.cannon_info`)))
  (bind _returnvalue (`|GetDataTableRow` _cannon_info_datatable _cannon_info_rowname)
    (:`then`
      (bind (_speed _duration) (break `/Game/Blueprints/Structs/Player/S_Player_Cannon_Info` _returnvalue))
      (set `self.speed` _speed)
      (set `self.time_left_alive` _duration))))

(event `self.ReceiveTick`
  (params (DeltaSeconds :type "Float (single-precision)"))
  (bind _time_left_alive (`self.time_left_alive`))
  (`self.K2_AddActorWorldOffset` (* (`self.direction`) (`self.speed`)))
  (set `self.time_left_alive` (- _time_left_alive DeltaSeconds))
  (if (<= _time_left_alive 0.0)
    (`self.K2_DestroyActor`)))

(fn `UserConstructionScript`)