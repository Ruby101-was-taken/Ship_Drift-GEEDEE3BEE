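; Player ship character that drives forward and backward and steers through axis input.
; BeginPlay reads movement and steering speeds from a data table row and sets the max walk speed.
; Gearing input eases a clamped engine speed into a signed speed with limited reverse, applied as mass-scaled forward force on CharacterMovement, with debug prints.
; Steer input adds controller yaw scaled by steering speed.
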(event `self.ReceiveBeginPlay`
  (bind (_player_movement_info_datatable _player_movement_info_rowname) (break `DataTableRowHandle` (`self.player_movement_info`)))
  ; On Start
  (bind _returnvalue (`|GetDataTableRow` _player_movement_info_datatable _player_movement_info_rowname)
    (:`then`
      (bind (_movement_speed _steering_speed) (break `/Game/Blueprints/Structs/Player/S_player-movement_info` _returnvalue))
      (set `self.movement_speed` _movement_speed)
      (set `self.steering_speed` _steering_speed)
      (set `CharacterMovementComponent.MaxWalkSpeed` (`self.movement_speed`) (`self.CharacterMovement`)))))

(event `InputAxis|Player_Gearing`
  (params (AxisValue :type "Float (single-precision)"))
  (bind _current_speed (`self.current_speed`))
  (bind _charactermovement (`self.CharacterMovement`))
  (bind _engine_speed (`self.engine_speed`))
  (bind _movement_speed (`self.movement_speed`))
  (bind _returnvalue (* (`self.GetActorForwardVector`) (* (`CharacterMovementComponent.Mass` _charactermovement) 4.0) _current_speed))
  ; Handle Acceleration
  (set `self.engine_speed` (`KismetMathLibrary.FClamp` (`KismetMathLibrary.FInterpTo` _engine_speed (`KismetMathLibrary.Abs` AxisValue) (`GameplayStatics.GetWorldDeltaSeconds`) 1.0) 0.25))
  (set `self.current_speed` (`KismetMathLibrary.FClamp` (* (`KismetMathLibrary.Lerp` 0.0 (`self.movement_speed`) _engine_speed) (`KismetMathLibrary.SignOfFloat` AxisValue)) (* _movement_speed -0.6) _movement_speed))
  ; Forward and Backwards
  (`CharacterMovementComponent.AddForce` _charactermovement _returnvalue)
  (`KismetSystemLibrary.PrintString` (`KismetStringLibrary.Conv_VectorToString` _returnvalue) true true (struct :`G` 0.66 :`B` 1.0 :`A` 1.0) 0.2 "Force")
  (`KismetSystemLibrary.PrintString` (`KismetStringLibrary.Conv_DoubleToString` _current_speed) true true (struct :`R` 1.0 :`G` 0.040452 :`A` 1.0) 0.2 "Acc")
  (`KismetSystemLibrary.PrintString` (`KismetStringLibrary.Conv_DoubleToString` (`self.engine_speed`)) true true (struct :`R` 0.169471 :`G` 1.0 :`B` 0.114506 :`A` 1.0) 0.2 "Input"))

(event `InputAxis|Player_Steer`
  (params (AxisValue :type "Float (single-precision)"))
  ; Turning left and right
  (`self.AddControllerYawInput` (* AxisValue (`self.steering_speed`))))

(fn `UserConstructionScript`)