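; BP_Player_CannonBall is a player cannonball projectile that travels along a set direction for a limited lifetime.
; Its Spawn event reads base speed, duration and damage from a CannonInfo data table row, increasing each by the passed-in fractional bonus.
; Tick offsets it without sweep by Direction times Speed per frame, unscaled by delta time, and destroys it when its lifetime expires.
; Damage is stored but not applied in these graphs.
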(event `Spawn`
  (params (damage :type "Float (double-precision)") (time :type "Float (double-precision)") (speed :type "Float (double-precision)"))
  (bind (_cannon_info_datatable _cannon_info_rowname) (break `DataTableRowHandle` (`self.cannon_info`)))
  (bind _returnvalue (`|GetDataTableRow` _cannon_info_datatable _cannon_info_rowname)
    (:`then`
      (bind (_speed _duration _damage) (break `/Game/Blueprints/Structs/Player/S_Player_Cannon_Info` _returnvalue))
      (set `self.speed` (+ (* speed _speed) _speed))
      (set `self.time_left_alive` (+ (* time _duration) _duration))
      (set `self.damage` (+ (* damage _damage) _damage)))))

(event `self.ReceiveTick`
  (params (DeltaSeconds :type "Float (single-precision)"))
  (bind _time_left_alive (`self.time_left_alive`))
  (`self.K2_AddActorWorldOffset` (* (`self.direction`) (`self.speed`)))
  (set `self.time_left_alive` (- _time_left_alive DeltaSeconds))
  (if (<= _time_left_alive 0.0)
    (`self.K2_DestroyActor`)))

(fn `UserConstructionScript`)