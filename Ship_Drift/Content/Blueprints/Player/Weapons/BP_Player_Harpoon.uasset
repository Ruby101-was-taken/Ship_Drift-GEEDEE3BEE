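; BP_Player_Harpoon is the player's harpoon projectile, fired toward a grapple point and later recalled.
; HarpoonOnToPosition stores the target, plays the attach sound and snaps the root to the player found at BeginPlay.
; While deployed, Tick eases it toward that point with VInterpTo and applies the grapple rotation.
; ReturnHarpoon re-arms the CanBeShot flag and parks it just below the world origin.
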(event `self.ReceiveBeginPlay`
  (bind _outactors (`GameplayStatics.GetAllActorsOfClass` "/Game/Blueprints/Player/BP_Player.BP_Player_C"))
  (set `self.player` (`|GetArrayItem` _outactors)))

(event `HarpoonOnToPosition`
  (params (position :type "Vector Structure (by ref)") (rotation :type "Rotator Structure (by ref)"))
  (if (`self.can_be_shot`)
    (set `self.grapple_point` position)
    (set `self.grapple_rotation` rotation)
    (set `self.can_be_shot` false)
    (`GameplayStatics.PlaySoundAtLocation` "/Game/Sound/SoundCue/A_Harpoon_Attach_Cue.A_Harpoon_Attach_Cue" (`self.K2_GetActorLocation`) (struct) 1.0 1.0 0.0 null null null null)
    (`SceneComponent.K2_SetWorldTransform` (`self.DefaultSceneRoot`) (`self.GetTransform` (`self.player`)) false false)))

(event `Return Harpoon`
  (if (not (`self.can_be_shot`))
    (set `self.can_be_shot` true)
    (`SceneComponent.K2_SetWorldTransform` (`self.DefaultSceneRoot`) (`KismetMathLibrary.MakeTransform` (0.0 0.0 -100.0)) false false)))

(event `self.ReceiveTick`
  (params (DeltaSeconds :type "Float (single-precision)"))
  (if (not (`self.can_be_shot`))
    (`SceneComponent.K2_SetWorldTransform` (`self.DefaultSceneRoot`) (`KismetMathLibrary.MakeTransform` (`KismetMathLibrary.VInterpTo` (`SceneComponent.K2_GetComponentLocation` (`self.DefaultSceneRoot`)) (`self.grapple_point`) DeltaSeconds 10.0) (`self.grapple_rotation`)) false false)))

(fn `UserConstructionScript`)