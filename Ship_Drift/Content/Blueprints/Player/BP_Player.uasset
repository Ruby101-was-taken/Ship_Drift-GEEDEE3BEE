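; Player character that drives with gearing and steering, fires sideways cannonballs with decaying recoil, and shoots a harpoon.
; Harpoon aim follows the clamped spring-arm camera, fanning line traces for tolerance before commanding the level's BP_Player_Harpoon.
; Health death costs a life, which resets health and position; losing all lives opens L_Test.
; Stats come from a data table, with skill-point-limited upgrades layered on as multipliers for movement and additive cannon modifiers.
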(event `self.Health.OnTakeDamagae`
  (params (DamageTaken :type "Float (double-precision)"))
  ;[0.15 0 0.0722 0.5] Health
  (`KismetSystemLibrary.PrintString` (`KismetStringLibrary.Conv_DoubleToString` (`/Game/Blueprints/Components/General/Health/BPC_health_component.health` (`self.Health`)))))

(event `self.Lives.OnLifeLost`
  (params (LivesLeft :type Integer))
  ;[0.15 0 0.0722 0.5] Health
  (`/Game/Blueprints/Components/General/Health/BPC_health_component.ResetHealth` (`self.Health`))
  (`self.K2_SetActorLocation` (0.0 0.0 0.0)))

(event `self.ReceiveBeginPlay`
  (bind (_player_movement_info_datatable _player_movement_info_rowname) (break `DataTableRowHandle` (`self.player_movement_info`)))
  ;[0 1 0.0235 0.5] On Start
  (bind _returnvalue (`|GetDataTableRow` _player_movement_info_datatable _player_movement_info_rowname)
    (:`then`
      (`self.SetPlayerAttributes` _returnvalue)
      (bind _outactors (`GameplayStatics.GetAllActorsOfClass` "/Game/Blueprints/Player/Weapons/BP_Player_Harpoon.BP_Player_Harpoon_C"))
      (set `self.player_harpoon` (`|GetArrayItem` _outactors)))))

(event `self.Health.OnDeath`
  ;[0.15 0 0.0722 0.5] Health
  (`/Game/Blueprints/Components/Player/BPC_player_lives_component.LoseLife` (`self.Lives`)))

(event `self.ReceiveAnyDamage`
  (params (Damage :type "Float (single-precision)") (DamageType :type "DamageType Object Reference") (InstigatedBy :type "Controller Object Reference") (DamageCauser :type "Actor Object Reference"))
  ;[0.15 0 0.0722 0.5] Health
  (`/Game/Blueprints/Components/General/Health/BPC_health_component.TakeDamage` (`self.Health`) Damage))

(event `self.Lives.OnAllLivesLost`
  ;[0.15 0 0.0722 0.5] Health
  ;; should be like death screen or main menu
  (`GameplayStatics.OpenLevel` "L_Test"))

(event `InputAxis|Player_Gearing`
  (params (AxisValue :type "Float (single-precision)"))
  ;[0.04127 0 1 0.5] Forward and Backwards
  (`self.AddMovementInput` (`self.GetActorForwardVector`) (* AxisValue (`self.movement_speed`)) true))

(event `self.ReceiveTick`
  (params (DeltaSeconds :type "Float (single-precision)"))
  (bind _cannon_cool_down (`self.cannon_cool_down`))
  (bind _cannon_recoil_direction (`self.cannon_recoil_direction`))
  ; On Update
  (if (`self.in_cannon_recoil`)
    (`self.LaunchCharacter` (* _cannon_recoil_direction DeltaSeconds))
    (set `self.cannon_recoil_direction` (`KismetMathLibrary.VLerp` _cannon_recoil_direction (0.0 0.0 0.0) (* DeltaSeconds (`self.cannon_recoil_momentum_lerp_alpha`))))
    (if (< (`KismetMathLibrary.VSize` _cannon_recoil_direction) 0.001)
      (set `self.in_cannon_recoil` false)))
  (if (not (<= _cannon_cool_down 0.0))
    (bind _output_get (set `self.cannon_cool_down` (- _cannon_cool_down DeltaSeconds)))
    (`KismetSystemLibrary.PrintString` (`KismetStringLibrary.Concat_StrStr` "Cannon Cool Down: " (`KismetStringLibrary.Conv_DoubleToString` _output_get)))))

(event `InputAxis|Player_Steer`
  (params (AxisValue :type "Float (single-precision)"))
  ;[0.04127 0 1 0.5] Turning left and right
  (`self.AddControllerYawInput` (* AxisValue (`self.steering_speed`))))

(event `InputAxis|Player_Shoot_Cannon`
  (params (AxisValue :type "Float (single-precision)"))
  (bind (_returnvalue_location _returnvalue_rotation _returnvalue_scale) (`KismetMathLibrary.BreakTransform` (`self.GetTransform`)))
  (bind _vector (`self.GetCannonMovementVector` (* AxisValue (`self.cannon_recoil_strength`))))
  ;[0 0 0 0.5] Shoot Cannon Recoil
  (if (and (!= AxisValue 0.0) (<= (`self.cannon_cool_down`) 0.0))
    (set `self.cannon_cool_down` (`self.base_cannon_cool_down`))
    (set `self.in_cannon_recoil` true)
    (set `self.cannon_recoil_direction` _vector)
    (bind _returnvalue (`|SpawnActorFromClass` "/Game/Blueprints/Player/Weapons/BP_Player_CannonBall.BP_Player_CannonBall_C" (`KismetMathLibrary.MakeTransform` (+ _returnvalue_location (* (`KismetMathLibrary.GetRightVector` _returnvalue_rotation) (* AxisValue -100.0))) _returnvalue_rotation _returnvalue_scale) "Undefined" "MultiplyWithRoot" null (`KismetMathLibrary.Normal` (* _vector -1.0)) null))
    (`/Game/Blueprints/Player/Weapons/BP_Player_CannonBall.Spawn` _returnvalue (`self.cannon_damage`) (`self.cannon_duration`) (`self.cannon_speed`))))

(event `InputAxisKey|MouseX`
  (params (AxisValue :type "Float (single-precision)"))
  (bind _springarm (`self.SpringArm`))
  (bind (_relativerotation_roll _relativerotation_pitch _relativerotation_yaw) (`KismetMathLibrary.BreakRotator` (`SceneComponent.RelativeRotation` _springarm)))
  (bind _returnvalue (+ _relativerotation_yaw AxisValue))
  ;[0.15 0.2435 0.01484 0.5] Camera Mouse Movement
  (if (< (`KismetMathLibrary.Abs` _returnvalue) (`self.harpoon_aim_range`))
    (`SceneComponent.K2_SetRelativeRotation` _springarm (`KismetMathLibrary.MakeRotator` 0.0 0.0 _returnvalue) false false)
    (else
      (`SceneComponent.K2_SetRelativeRotation` _springarm (`KismetMathLibrary.MakeRotator` 0.0 0.0 (* (`KismetMathLibrary.SignOfFloat` _returnvalue) (`self.harpoon_aim_range`))) false false))))

(event `InputAction|Player_Harpoon_Shoot`
  (params (Key :type "Key Structure"))
  (bind (_returnvalue_location _returnvalue_rotation) (`KismetMathLibrary.BreakTransform` (`self.GetTransform`)))
  (bind (_returnvalue_location_2 _returnvalue_rotation_2) (`KismetMathLibrary.BreakTransform` (`self.GetTransform`)))
  (:`Pressed`
    (for _index (range (+ (`self.harpoon_tolerance`) 1))
      (bind (_outhit _returnvalue) (`KismetSystemLibrary.LineTraceSingleForObjects` :`Start` _returnvalue_location_2 :`End` (+ _returnvalue_location_2 (* (`KismetMathLibrary.Normal` (`KismetMathLibrary.GreaterGreater_VectorRotator` (`KismetMathLibrary.MakeVector` (.x (`SceneComponent.GetForwardVector` (`self.Camera`))) (.y (`SceneComponent.GetForwardVector` (`self.Camera`)))) (`KismetMathLibrary.MakeRotator` 0.0 0.0 (* (select `bool` (== _index 0) :`false` (select `bool` (== (mod _index 2) 0) :`false` -1.0 :`true` 1.0 :!type "Float (single-precision)")) (/ _index 2))))) (`self.harpoon_length`))) :`ObjectTypes` (`self.Object Types`) :`DrawDebugType` "Persistent"))
      (if _returnvalue
        (`/Game/Blueprints/Player/Weapons/BP_Player_Harpoon.HarpoonOnToPosition` (`self.player_harpoon`) (`.ImpactPoint` (`GameplayStatics.BreakHitResult` _outhit)) _returnvalue_rotation)
        (break)))))

(event `HarpoonPull`
  (params (Velocity :type "Vector Structure"))
  (`self.LaunchCharacter` Velocity))

(event `InputAction|Player_Harpoon_Return`
  (params (Key :type "Key Structure"))
  (:`Pressed`
    (`/Game/Blueprints/Player/Weapons/BP_Player_Harpoon.Return Harpoon` (`self.player_harpoon`))))

(event `Add Upgrade`
  (params (upgrade_name :type String))
  (bind (_player_movement_info_datatable _player_movement_info_rowname) (break `DataTableRowHandle` (`self.player_movement_info`)))
  (if (not (`KismetArrayLibrary.Array_Contains` (`self.player_upgrades`) upgrade_name))
    (`KismetArrayLibrary.Array_Add` (`self.player_upgrades`) upgrade_name)
    (bind _returnvalue (`|GetDataTableRow` (`self.player_upgrade_table`) (`KismetStringLibrary.Conv_StringToName` upgrade_name))
      (:`then`
        (bind _returnvalue_2 (+ (`.skill_points_25_3B422A1C46E775C1B065618DF2D7B62F` (break `/Game/Blueprints/Structs/Upgrades/S_modifier` _returnvalue)) (`self.used_skill_points`)))
        (if (> _returnvalue_2 (`self.max_skill_points`))
          (`KismetSystemLibrary.PrintString` "not enough points")
          (else
            (set `self.used_skill_points` _returnvalue_2)
            (bind _returnvalue_3 (`|GetDataTableRow` _player_movement_info_datatable _player_movement_info_rowname :!label _label)
              (:`then`
                (`self.SetPlayerAttributes` _returnvalue_3)
                (`KismetSystemLibrary.PrintString` (`KismetStringLibrary.Conv_IntToString` (`self.used_skill_points`)))))))))))

(event `Remove Upgrade`
  (params (upgrade_name :type String))
  (bind _returnvalue (`KismetArrayLibrary.Array_RemoveItem` (`self.player_upgrades`) upgrade_name))
  (if _returnvalue
    (bind _returnvalue_2 (`|GetDataTableRow` (`self.player_upgrade_table`) (`KismetStringLibrary.Conv_StringToName` upgrade_name))
      (:`then`
        (set `self.used_skill_points` (- (`self.used_skill_points`) (`.skill_points_25_3B422A1C46E775C1B065618DF2D7B62F` (break `/Game/Blueprints/Structs/Upgrades/S_modifier` _returnvalue_2))))
        (goto _label)))))

(fn `GetCannonMovementVector`
  (params (axis :type "Float (double-precision)"))
  (returns (vector :type "Vector Structure"))
  (bind (_returnvalue_x _returnvalue_y _returnvalue_z) (`KismetMathLibrary.BreakVector` (`KismetMathLibrary.MakeVector` axis)))
  (bind (_returnvalue_location _returnvalue_rotation) (`KismetMathLibrary.BreakTransform` (`self.GetTransform`)))
  (return (+ (* _returnvalue_x (`KismetMathLibrary.GetRightVector` _returnvalue_rotation)) (* _returnvalue_z (`KismetMathLibrary.GetForwardVector` _returnvalue_rotation)))))

(fn `SetPlayerAttributes`
  (params (player_data :type "/Game/Blueprints/Structs/Player/S_player-movement_info Structure (by ref)"))
  (bind (_movement_speed _steering_speed _cannon_recoil_strength _cannon_recoil_momentum_lerp_alpha _harpoon_tolerance _harpoon_length _harpoon_pull_strength) (break `/Game/Blueprints/Structs/Player/S_player-movement_info` player_data))
  (bind (_movement_speed_2 _steering_speed_2 _cannon_recoil_strength_2 _cannon_recoil_momentum_lerp_alpha_2 _harpoon_tolerance_2 _harpoon_length_2 _harpoon_pull_strength_2) (break `/Game/Blueprints/Structs/Player/S_player-movement_info` player_data))
  (bind _player_upgrade_table (`self.player_upgrade_table`))
  (bind _output_get (set `self.movement_speed` _movement_speed_2))
  (set `CharacterMovementComponent.MaxWalkSpeed` _output_get (`self.CharacterMovement`))
  (set `self.steering_speed` _steering_speed_2)
  (set `self.cannon_recoil_strength` _cannon_recoil_strength_2)
  (set `self.cannon_recoil_momentum_lerp_alpha` _cannon_recoil_momentum_lerp_alpha_2)
  (set `self.harpoon_tolerance` _harpoon_tolerance_2)
  (set `self.harpoon_length` _harpoon_length_2)
  (set `self.harpoon_pull_strength` _harpoon_pull_strength_2)
  (set `self.base_cannon_cool_down` 1.0)
  (bind _outrownames (`DataTableFunctionLibrary.GetDataTableRowNames` _player_upgrade_table))
  (for _array_element _outrownames
    (for _array_element_2 (`self.player_upgrades`)
      (if (== (`KismetStringLibrary.Conv_NameToString` _array_element) _array_element_2)
        (bind _returnvalue (`|GetDataTableRow` _player_upgrade_table _array_element)
          (:`then`
            (bind (_movement _cannon) (break `/Game/Blueprints/Structs/Upgrades/S_modifier` _returnvalue))
            (bind (_harpoon_pull_strength_3 _harpoon_length_3 _harpoon_tolerance_3 _cannon_recoil_momentum_lerp_alpha_3 _cannon_recoil_strength_3 _steering_speed_3 _movement_speed_3) (break `/Game/Blueprints/Structs/Upgrades/Movement/S_movement_modifer` _movement))
            (set `self.harpoon_pull_strength` (+ (* _harpoon_pull_strength_3 _harpoon_pull_strength) (`self.harpoon_pull_strength`)))
            (set `self.harpoon_length` (+ (* _harpoon_length_3 _harpoon_length) (`self.harpoon_length`)))
            (set `self.harpoon_tolerance` (`KismetMathLibrary.FTrunc` (+ (* _harpoon_tolerance_3 _harpoon_tolerance) (`self.harpoon_tolerance`))))
            (set `self.cannon_recoil_momentum_lerp_alpha` (+ (* _cannon_recoil_momentum_lerp_alpha_3 _cannon_recoil_momentum_lerp_alpha) (`self.cannon_recoil_momentum_lerp_alpha`)))
            (set `self.cannon_recoil_strength` (+ (* _cannon_recoil_strength_3 _cannon_recoil_strength) (`self.cannon_recoil_strength`)))
            (set `self.steering_speed` (+ (* _steering_speed_3 _steering_speed) (`self.steering_speed`)))
            (bind _output_get_2 (set `self.movement_speed` (+ (* _movement_speed_3 _movement_speed) (`self.movement_speed`))))
            (set `CharacterMovementComponent.MaxWalkSpeed` _output_get_2 (`self.CharacterMovement`))
            (bind (_speed _duration _damage _cooldown) (break `/Game/Blueprints/Structs/Upgrades/Cannon/S_Cannon_Modifier` _cannon))
            (bind _returnvalue_2 (+ _speed (`self.cannon_speed`)))
            (if (> _returnvalue_2 0.0)
              (set `self.cannon_speed` _returnvalue_2))
            (set `self.cannon_duration` (+ _duration (`self.cannon_duration`)))
            (set `self.cannon_damage` (+ _damage (`self.cannon_damage`)))
            (set `self.base_cannon_cool_down` (+ _cooldown (`self.base_cannon_cool_down`))))
          (:`RowNotFound`
            (`KismetSystemLibrary.PrintString` "fake upgrade")))))))

(fn `UserConstructionScript`)