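; Score manager that tracks the scrap currency, both total and per level, plus a pausable level timer.
; All scrap changes funnel through AddScrap, which fires OnIncrementScrap; SimpleReset subtracts the level's scrap, while Reset clears level scrap and timer.
; Level-end rewards grant bonus scrap for fast times and high collection.
; Life and skill point prices escalate per query, using half the current scrap or a fixed step, whichever is higher.
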(event `IncermentScrap`
  (params (by :type Integer :default 1))
  (`self.AddScrap` by))

(event `/Game/Blueprints/Interfaces/BPI_Resetable.SimpleReset`
  (`self.IncermentScrap` (* (`self.scrap_this_level`) -1)))

(event `/Game/Blueprints/Interfaces/BPI_Resetable.Reset`
  (params (level_type :type "/Game/Blueprints/Enum/Levels/Types/E_Level_Types Enum" :default "NewEnumerator0") (wind :type "Vector Structure") (weather :type "/Game/Blueprints/Enum/Levels/Types/E_Weather_Types Enum" :default "NewEnumerator0") (test_type :type "/Game/Blueprints/Enum/Testing/E_Tester_Type Enum" :default "NewEnumerator0"))
  (set `self.scrap_this_level` 0)
  (set `self.timer` 0.0)
  (set `self.pause_timer` false))

(event `self.ReceiveTick`
  (params (DeltaSeconds :type "Float (single-precision)"))
  (if (not (`self.pause_timer`))
    (set `self.timer` (+ DeltaSeconds (`self.timer`)))))

(fn `AddScrap`
  (params (new_scrap :type Integer))
  (bind _scrap (`self.Scrap`))
  (set `self.Scrap` (+ new_scrap _scrap))
  (set `self.scrap_this_level` (+ new_scrap (`self.scrap_this_level`)))
  (`KismetSystemLibrary.PrintString` (`KismetStringLibrary.Concat_StrStr` "Scrap: " (`KismetStringLibrary.Conv_IntToString` _scrap)))
  (`self.On Increment Scrap`))

(fn `DeIncrementScrap`
  (params (scrap_to_subtract :type Integer))
  (`self.IncermentScrap` (* scrap_to_subtract -1)))

(fn `GetLifePrice`
  (returns (price :type Integer))
  (bind _output_get (set `self.last_life_price` (`KismetMathLibrary.Max` (/ (`self.Scrap`) 2) (+ (`self.last_life_price`) 10))))
  (return _output_get))

(fn `GetSkillPointPrice`
  (returns (price :type Integer))
  (bind _output_get (set `self.last_skill_point_price` (`KismetMathLibrary.Max` (/ (`self.Scrap`) 2) (+ (`self.last_skill_point_price`) 10))))
  (return _output_get))

(fn `GetTimerString`
  (returns (timer_string :type String))
  (bind _timer (`self.timer`))
  (return (`KismetTextLibrary.Conv_TextToString` (`|FormatText` "{MM}:{SS}:{DDD}" (`KismetTextLibrary.Conv_IntToText` (/ _timer 60) false true 2) (`KismetTextLibrary.Conv_IntToText` (mod (`KismetMathLibrary.FTrunc` _timer) 60) false true 2) (`KismetTextLibrary.Conv_IntToText` (`KismetMathLibrary.FTrunc` (* (mod _timer 1.0) 1000.0)) false true 3 3)))))

(fn `GiveEndOfLevelRewards`
  (returns (time_scrap :type Integer) (scrap_scrap :type Integer))
  (locals (timer_bonus :type Integer :default 0) (scrap_bonus :type Integer))
  ; Timer Bonus
  (bind _output_get (set `local.timer_bonus` (`KismetMathLibrary.FTrunc` (`KismetMathLibrary.FMax` (- 90.0 (`self.timer`))))))
  (`self.AddScrap` _output_get)
  ; Scrap collection bonus
  (bind _output_get_2 (set `local.scrap_bonus` (`KismetMathLibrary.Max` (/ (- (`self.scrap_this_level`) 50) 2))))
  (`self.AddScrap` _output_get_2)
  (return (`local.timer_bonus`) (`local.scrap_bonus`)))

(fn `UserConstructionScript`)