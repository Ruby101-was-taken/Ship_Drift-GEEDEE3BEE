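; Level manager that resets the level on BeginPlay or when ResetLevel fires, controlling level type, weather and wind.
; ResetLevel fires a dispatcher, sends current values to every BPI_Resetable actor, then randomises the next set.
; Recursive picks exclude the current level type and two reserved types; weather's check and assignment roll separately, so it can repeat.
; Wind is a random positive-axis vector, scaled and doubled for one weather type.
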(event `self.ReceiveBeginPlay`
  (set `self.next_level_type` (`self.beginning_level_type`))
  (`self.Reset Level`))

(event `Reset Level`
  (`KismetSystemLibrary.PrintString` (`KismetStringLibrary.Concat_StrStr` "Level Type: " (`|GetEnumeratorNameAsString` (`self.next_level_type`))) true true (struct :`G` 1.0 :`B` 0.093925 :`A` 1.0) 30.0)
  (`KismetSystemLibrary.PrintString` (`KismetStringLibrary.Concat_StrStr` "Weather Type: " (`|GetEnumeratorNameAsString` (`self.next_weather_type`))) true true (struct :`G` 1.0 :`B` 0.093925 :`A` 1.0) 30.0)
  (`self.On Level Reset`)
  (bind _outactors (`GameplayStatics.GetAllActorsWithInterface` "/Game/Blueprints/Interfaces/BPI_Resetable.BPI_Resetable_C"))
  (for _array_element _outactors
    (message `/Game/Blueprints/Interfaces/BPI_Resetable.Reset` _array_element (`self.next_level_type`) (`self.next_wind_direction`) (`self.next_weather_type`)))
  (`self.RandomiseLevelType`)
  (`self.RandomiseWeatherType`))

(fn `RandomiseLevelType`
  (locals (attempted_level_type :type "/Game/Blueprints/Enum/Levels/Types/E_Level_Types Enum"))
  (bind _attempted_level_type (`local.attempted_level_type`))
  (set `local.attempted_level_type` (cast `/Game/Blueprints/Enum/Levels/Types/E_Level_Types` (`KismetMathLibrary.Conv_IntToByte` (`KismetMathLibrary.RandomInteger` (enumcount `/Game/Blueprints/Enum/Levels/Types/E_Level_Types`)))))
  (if (and (`|EnumInequality` (`self.next_level_type`) _attempted_level_type) (`|EnumInequality` _attempted_level_type "NewEnumerator0") (`|EnumInequality` _attempted_level_type "NewEnumerator7"))
    (set `self.next_level_type` _attempted_level_type)
    (else
      (`self.RandomiseLevelType`))))

(fn `RandomiseWeatherType`
  (bind _returnvalue (cast `/Game/Blueprints/Enum/Levels/Types/E_Weather_Types` (`KismetMathLibrary.Conv_IntToByte` (`KismetMathLibrary.RandomInteger` (enumcount `/Game/Blueprints/Enum/Levels/Types/E_Weather_Types`)))))
  (if (not (`|EnumEquality` (`self.next_weather_type`) _returnvalue))
    (set `self.next_weather_type` _returnvalue)
    (`self.RandomiseWind`)
    (else
      (`self.RandomiseWeatherType`))))

(fn `RandomiseWind`
  (locals (wind_dir :type "Vector Structure"))
  (bind _output_get (set `local.wind_dir` (`KismetMathLibrary.MakeVector` (`KismetMathLibrary.RandomFloatInRange` 0.0 1.0) (`KismetMathLibrary.RandomFloatInRange` 0.0 1.0) (`KismetMathLibrary.RandomFloatInRange` 0.0 1.0))))
  (set `self.next_wind_direction` (* (`KismetMathLibrary.Normal` _output_get) (`self.wind_scale`) (`KismetMathLibrary.SelectFloat` 2.0 1.0 (`|EnumEquality` (`self.next_weather_type`) "NewEnumerator1")))))

(fn `UserConstructionScript`)