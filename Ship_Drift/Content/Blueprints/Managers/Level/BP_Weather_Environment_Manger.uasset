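; Weather environment manager that adjusts the level's fog and sunlight to match the weather state.
; On BeginPlay it caches the first ExponentialHeightFog and DirectionalLight actors found in the level.
; Its Reset event takes a Weather value (Clear, Rainy or Foggy) and uses it to select the matching fog density and light color variables, then applies them to those actors.
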(event `self.ReceiveBeginPlay`
  ; Get all References
  (bind _outactors (`GameplayStatics.GetAllActorsOfClass` "/Script/Engine.ExponentialHeightFog"))
  (set `self.fog` (`|GetArrayItem` _outactors))
  (bind _outactors_2 (`GameplayStatics.GetAllActorsOfClass` "/Script/Engine.DirectionalLight"))
  (set `self.light` (`|GetArrayItem` _outactors_2)))

(event `/Game/Blueprints/Interfaces/BPI_Resetable.Reset`
  (params (level_type :type "/Game/Blueprints/Enum/Levels/Types/E_Level_Types Enum" :default "NewEnumerator0") (wind :type "Vector Structure") (weather :type "/Game/Blueprints/Enum/Levels/Types/E_Weather_Types Enum" :default "NewEnumerator0"))
  ; On Level Reset - Apply Changes based on Weather
  (`self.Set Fog Attributes` weather)
  (`self.Set Light Attributes` weather))

(fn `Set Fog Attributes`
  (params (Index :type "/Game/Blueprints/Enum/Levels/Types/E_Weather_Types Enum" :default "NewEnumerator0"))
  (`ExponentialHeightFogComponent.SetFogDensity` (`ExponentialHeightFog.Component` (`self.fog`)) (select `/Game/Blueprints/Enum/Levels/Types/E_Weather_Types` Index :`NewEnumerator0` (`self.clear_density`) :`NewEnumerator1` (`self.rainy_density`) :`NewEnumerator2` (`self.foggy_density`))))

(fn `Set Light Attributes`
  (params (Index :type "/Game/Blueprints/Enum/Levels/Types/E_Weather_Types Enum" :default "NewEnumerator0"))
  (`LightComponent.SetLightColor` (`Light.LightComponent` (`self.light`)) (select `/Game/Blueprints/Enum/Levels/Types/E_Weather_Types` Index :`NewEnumerator0` (`self.clear_light_colour`) :`NewEnumerator1` (`self.rainy_light_colour`) :`NewEnumerator2` (`self.foggy_light_colour`)) true))

(fn `UserConstructionScript`)