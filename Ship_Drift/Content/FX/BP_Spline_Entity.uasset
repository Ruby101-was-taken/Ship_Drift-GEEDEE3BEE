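; BP_Spline_Entity is an actor that moves along the spline of a referenced actor, carrying a configurable static mesh.
; The construction script applies the chosen mesh.
; On BeginPlay, a timeline with play rate set from TimeToComplete drives an alpha from zero to full spline length.
; Each update places and rotates the actor to match the spline's world-space location and rotation at that distance.
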(event `self.ReceiveBeginPlay`
  (`self.Move Obj`))

(event `Move Obj`
  (bind _spline (`/Game/FX/BP_Spline_Path.Spline` (`self.Spline_Ref`)))
  (`TimelineComponent.SetPlayRate` (`self.T_Move`) (/ 1.0 (`self.Time_To_Complete`)))
  (bind (_direction _move_track) (`Timeline|T_Move`)
    (:`Update`
      (bind _returnvalue (`KismetMathLibrary.Lerp` 0.0 (`SplineComponent.GetSplineLength` _spline) _move_track))
      (`self.K2_SetActorLocationAndRotation` (`SplineComponent.GetLocationAtDistanceAlongSpline` _spline _returnvalue "World") (`SplineComponent.GetRotationAtDistanceAlongSpline` _spline _returnvalue "World")))))

(fn `UserConstructionScript`
  (`StaticMeshComponent.SetStaticMesh` (`self.Actor`) (`self.New_Actor`)))